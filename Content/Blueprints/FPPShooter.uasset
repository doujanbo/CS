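; First-person shooter player character that moves, looks, fires and switches between a rifle and a launcher.
; BeginPlay creates both guns and shows the first, while input axes drive movement and view from the control rotation.
; Fire press and release forward to the current gun, and Equip stops firing, cycles the gun index by toggling visibility and plays an equip montage.
; GetShooterLoation exposes the camera's world position.
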(event `InputAction|Equip`
  (params (Key :type "Key Structure"))
  (:`Pressed`
    (`self.SwitchWeapon`)))

(event `self.ReceiveBeginPlay`
  ;[1 1 1] 添加枪
  (`self.CreateGun` "/Game/Blueprints/Rifle.Rifle_C")
  (`self.CreateGun` "/Game/Blueprints/Launcher.Launcher_C")
  (set `self.CurrentIndex` 0)
  (`self.SetActorHiddenInGame` (`self.GetCurrentGun`) false))

(event `InputAxis|MoveForward`
  (params (AxisValue :type "Float (single-precision)"))
  ;[1 1 1] 移动
  (`self.AddMovementInput` (`KismetMathLibrary.Conv_RotatorToVector` (`self.GetControlRotation`)) AxisValue))

(event `InputAxis|MoveRight`
  (params (AxisValue :type "Float (single-precision)"))
  ;[1 1 1] 移动
  (`self.AddMovementInput` (`KismetMathLibrary.Conv_RotatorToVector` (`KismetMathLibrary.ComposeRotators` (`self.GetControlRotation`) (`KismetMathLibrary.MakeRotator` 0.0 0.0 90.0))) AxisValue))

(event `InputAxis|Turn`
  (params (AxisValue :type "Float (single-precision)"))
  ;[1 1 1] 视口角度
  (`self.AddControllerYawInput` AxisValue))

(event `InputAxis|LookUp`
  (params (AxisValue :type "Float (single-precision)"))
  ;[1 1 1] 视口角度
  (`self.AddControllerPitchInput` AxisValue))

(event `InputAction|Fire`
  (params (Key :type "Key Structure"))
  ;[1 1 1] 播放射击动画，添加射击特效
  (:`Pressed`
    (`self.StartFire`))
  (:`Released`
    (`self.EndFire`)))

(fn `EndFire`
  (`/Game/Blueprints/Gun.EndFire` (`self.GetCurrentGun`)))

(fn `GetShooterLoation`
  (returns (Loation :type "Vector Structure"))
  (return (`SceneComponent.K2_GetComponentLocation` (`self.Camera`))))

(fn `StartFire`
  (`/Game/Blueprints/Gun.StartFire` (`self.GetCurrentGun`)))

(fn `SwitchWeapon`
  (`self.EndFire`)
  (`self.SetActorHiddenInGame` (`self.GetCurrentGun`) true)
  (set `self.CurrentIndex` (mod (+ (`self.CurrentIndex`) 1) (`KismetArrayLibrary.Array_Length` (`self.Guns`))))
  (`self.SetActorHiddenInGame` (`self.GetCurrentGun`) false)
  (`self.PlayAnimMontage` "/Game/Blueprints/FppEquip_Montage.FppEquip_Montage"))

(fn `UserConstructionScript`)