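; Gun actor that gives its owning character an automatic hitscan rifle.
; StartFire plays the owner's fire montage, attaches a muzzle flash, fires immediately and repeats ShootOnce on a looping timer until EndFire clears all three.
; ShootOnce line-traces from the owner's camera along the control rotation, leaving persistent debug lines, and applies fixed damage only to RobotShooter hits.
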(fn `EndFire`
  (if (`self.IsInFire`)
    (set `self.IsInFire` false)
    (`KismetSystemLibrary.K2_ClearTimer` null "ShootOnce")
    (`Character.StopAnimMontage` (`self.GunOwner`) "/Game/Blueprints/FppRifleFire_Montage.FppRifleFire_Montage")
    (`ActorComponent.K2_DestroyComponent` (`self.FireEffects`))))

(fn `ShootOnce`
  (bind _returnvalue (`SceneComponent.K2_GetComponentLocation` (`/Game/Blueprints/FPPShooter.Camera` (`self.GunOwner`))))
  (bind (_outhit _returnvalue_2) (`KismetSystemLibrary.LineTraceSingle` :`Start` _returnvalue :`End` (+ (* (`KismetMathLibrary.Normal` (`KismetMathLibrary.GetForwardVector` (`Pawn.GetControlRotation` (`self.GunOwner`)))) 1500.0) _returnvalue) :`TraceChannel` "TraceTypeQuery1" :`DrawDebugType` "Persistent"))
  (if _returnvalue_2
    (bind _asrobot_shooter (cast `/Game/Blueprints/RobotShooter` (`.HitActor` (`GameplayStatics.BreakHitResult` _outhit))))
    (`/Game/Blueprints/RobotShooter.TakeDamage` _asrobot_shooter 20.0)))

(fn `StartFire`
  (`|ExecutionSequence`
    (:`then_0`
      (`Character.PlayAnimMontage` (`self.GunOwner`) "/Game/Blueprints/FppRifleFire_Montage.FppRifleFire_Montage" 1.0 "None")
      (bind _returnvalue (`GameplayStatics.SpawnEmitterAttached` "/Game/Assets/Effects/ParticleSystems/Weapons/AssaultRifle/Muzzle/P_AssaultRifle_MF.P_AssaultRifle_MF" (`self.Muzzle`)))
      (set `self.FireEffects` _returnvalue))
    (:`then_1`
      (`self.ShootOnce`)
      (`KismetSystemLibrary.K2_SetTimer` null "ShootOnce" 0.2 true))
    (:`then_2`
      (set `self.IsInFire` true))))

(fn `UserConstructionScript`)