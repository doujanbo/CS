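; Rifle weapon that gives its GunOwner automatic hitscan fire against Shooter targets.
; StartFire plays the firing montage, attaches a muzzle flash, fires immediately and repeats ShootOnce on a looping timer until EndFire clears all three.
; ShootOnce line-traces on the Camera channel along the owner's shoot direction and damages any Shooter hit.
; Leftover debugging draws persistent trace lines and prints a message on a miss.
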(fn `EndFire`
  (if (`self.IsInFire`)
    (set `self.IsInFire` false)
    (`KismetSystemLibrary.K2_ClearTimer` null "ShootOnce")
    (`Character.StopAnimMontage` (`self.GunOwner`) "/Game/Blueprints/FppRifleFire_Montage.FppRifleFire_Montage")
    (`ActorComponent.K2_DestroyComponent` (`self.FireEffects`))))

(fn `ShootOnce`
  (bind _loation (`/Game/Blueprints/Shooter.GetShooterLoation` (`self.GunOwner`)))
  (bind (_outhit _returnvalue) (`KismetSystemLibrary.LineTraceSingle` _loation (+ (* (`KismetMathLibrary.Normal` (`/Game/Blueprints/Shooter.GetShootDirection` (`self.GunOwner`))) 1500.0) _loation) "TraceTypeQuery2" false (`|MakeArray` (`self.GunOwner`) :!type "Actor Object Reference") "Persistent"))
  (if _returnvalue
    (bind _asshooter (cast `/Game/Blueprints/Shooter` (`.HitActor` (`GameplayStatics.BreakHitResult` _outhit))))
    (`/Game/Blueprints/Shooter.TakeDamage` _asshooter 20.0)
    (else
      (`KismetSystemLibrary.PrintString` "Hello"))))

(fn `StartFire`
  (`|ExecutionSequence`
    (:`then_0`
      (`Character.PlayAnimMontage` (`self.GunOwner`) "/Game/Blueprints/FppRifleFire_Montage.FppRifleFire_Montage" 1.0 "None")
      (bind _returnvalue (`GameplayStatics.SpawnEmitterAttached` "/Game/Assets/Effects/ParticleSystems/Weapons/AssaultRifle/Muzzle/P_AssaultRifle_MF.P_AssaultRifle_MF" (`self.Muzzle`)))
      (set `self.FireEffects` _returnvalue))
    (:`then_1`
      (`self.ShootOnce`)
      (`KismetSystemLibrary.K2_SetTimer` null "ShootOnce" 0.2 true))
    (:`then_2`
      (set `self.IsInFire` true))))

(fn `UserConstructionScript`
  (`parent.UserConstructionScript`))