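; Shooter is a pawn Blueprint that tracks health and handles its own death.
; TakeDamage subtracts from Health, then detaches the pawn from its controller pending destroy once IsDead finds health at or below zero.
; GetShooterLoation returns only a zero vector, and the event graph and construction script hold no logic.
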(fn `GetShooterLoation`
  (returns (Loation :type "Vector Structure"))
  (return (0.0 0.0 0.0)))

(fn `IsDead`
  (returns (Dead :type Boolean))
  (return (<= (`self.Health`) 0.0)))

(fn `TakeDamage`
  (params (Damage :type "Float (double-precision)"))
  (set `self.Health` (- (`self.Health`) Damage))
  (if (`self.IsDead`)
    (`self.DetachFromControllerPendingDestroy`)))

(fn `UserConstructionScript`)